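; Animation notify that plays a footstep sound matching the surface under the player character.
; On notify, it traces downward along the character's up axis on the Visibility channel and switches on the hit physical material's surface type to pick the sound.
; It always traces from player 0 rather than the notifying mesh's owner, plays audio as non-spatial 2D, and stays silent without a valid physical material.
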(fn `MakeFootstep`
  (bind _returnvalue (`GameplayStatics.GetPlayerCharacter` 0))
  (bind _returnvalue_2 (`Actor.K2_GetActorLocation` _returnvalue))
  (bind _outhit (`KismetSystemLibrary.LineTraceSingle` _returnvalue_2 (+ _returnvalue_2 (* (`Actor.GetActorUpVector` _returnvalue) -200.0)) "TraceTypeQuery1"))
  (if (`KismetSystemLibrary.IsValid` (`.PhysMat` (`GameplayStatics.BreakHitResult` _outhit)))
    (switch `EPhysicalSurface` (`PhysicalMaterial.SurfaceType` (`.PhysMat` (`GameplayStatics.BreakHitResult` _outhit)))
      (:`SurfaceType1`
        (`GameplayStatics.PlaySound2D` "/Game/Audio/Cues/A_GrassFootstep.A_GrassFootstep" 1.0 1.0 0.0 null null))
      (:`SurfaceType2`
        (`GameplayStatics.PlaySound2D` "/Game/Audio/Cues/A_DeepFootstep.A_DeepFootstep" 1.0 1.0 0.0 null null))
      (:`SurfaceType3`
        (`GameplayStatics.PlaySound2D` "/Game/Audio/Cues/A_SandFootstep.A_SandFootstep" 1.0 1.0 0.0 null null))
      (:`SurfaceType4`
        (`GameplayStatics.PlaySound2D` "/Game/Audio/Cues/A_MudFootstep.A_MudFootstep" 1.0 1.0 0.0 null null))
      (:`SurfaceType5`
        (`GameplayStatics.PlaySound2D` "/Game/Audio/Cues/A_GravelFootstep.A_GravelFootstep" 1.0 1.0 0.0 null null))
      (:`SurfaceType6`
        (`GameplayStatics.PlaySound2D` "/Game/Audio/Cues/A_LeavesFootstep.A_LeavesFootstep" 1.0 1.0 0.0 null null))
      (:`SurfaceType7`
        (`GameplayStatics.PlaySound2D` "/Game/Audio/Cues/A_ConcreteFootstep.A_ConcreteFootstep" 1.0 1.0 0.0 null null)))))

(fn `Received_Notify`
  (params (MeshComp :type "SkeletalMeshComponent Object Reference") (Animation :type "AnimSequenceBase Object Reference") (EventReference :type "AnimNotifyEventReference Structure (by ref)"))
  (returns (ReturnValue :type Boolean))
  (`self.MakeFootstep`)
  (return false))