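; BP_Flute is an equippable tool that emits an "Escape"-tagged AI noise at the player's location when used.
; Use runs the parent logic, makes the noise, starts a cooldown timer and calls Play for the melody sound and Niagara effect.
; Use during cooldown only plays an alternate sound and effect, with no noise.
; Both effects spawn at the flute, rotated relative to the player's facing.
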(event `self.ReceiveBeginPlay`
  (`parent.ReceiveBeginPlay`))

(fn `Equip`
  (`parent.Equip`))

(fn `Play`
  (`NiagaraFunctionLibrary.SpawnSystemAtLocation` "/Game/VFX/NS_FluteMelody.NS_FluteMelody" (`self.K2_GetActorLocation`) (`KismetMathLibrary.MakeRotator` (.roll (`self.K2_GetActorRotation` (`GameplayStatics.GetPlayerCharacter` 0))) (.pitch (`self.K2_GetActorRotation` (`GameplayStatics.GetPlayerCharacter` 0))) (+ (.yaw (`self.K2_GetActorRotation` (`GameplayStatics.GetPlayerCharacter` 0))) -90.0)))
  (`GameplayStatics.PlaySound2D` "/Game/Audio/Waves/pan-flute-long-sustain_C.pan-flute-long-sustain_C" 1.0 1.0 0.0 null null))

(fn `ResetCoolDown`
  (set `self.IsOnCoolDown` false))

(fn `Unequip`
  (`parent.Unequip`))

(fn `Use`
  (bind _returnvalue (`GameplayStatics.GetPlayerPawn` 0))
  (if (`self.IsOnCoolDown`)
    (`NiagaraFunctionLibrary.SpawnSystemAtLocation` "/Game/VFX/NS_CDFluteMelody.NS_CDFluteMelody" (`self.K2_GetActorLocation`) (`KismetMathLibrary.MakeRotator` (.roll (`self.K2_GetActorRotation` (`GameplayStatics.GetPlayerCharacter` 0))) (.pitch (`self.K2_GetActorRotation` (`GameplayStatics.GetPlayerCharacter` 0))) (+ (.yaw (`self.K2_GetActorRotation` (`GameplayStatics.GetPlayerCharacter` 0))) -90.0)))
    (`GameplayStatics.PlaySound2D` "/Game/Audio/Waves/pan-flute-wet-melody_126bpm_C_minor.pan-flute-wet-melody_126bpm_C_minor" 1.0 1.0 0.0 null null)
    (else
      (`parent.Use`)
      (`self.MakeNoise` 1.0 _returnvalue (`self.K2_GetActorLocation` _returnvalue) 1000.0 "Escape")
      (`KismetSystemLibrary.K2_SetTimer` null "ResetCoolDown" (`self.CoolDown`))
      (set `self.IsOnCoolDown` true)
      (`self.Play`))))

(fn `UserConstructionScript`
  (`parent.UserConstructionScript`))