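; BP_Torch is a hold-type tool whose hinged top opens and closes, with a heat source and Niagara fire effect.
; Use toggles heat and fire based on IsOpen, then calls a dispatcher that flips the state and swings the top via a timeline.
; Equip and Unequip rescale the mesh and open or close the top through that dispatcher, without touching heat or fire themselves.
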(event `self.ReceiveBeginPlay`
  (`parent.ReceiveBeginPlay`)
  (`HeatSourceComponent.Init` (`self.HeatSource`))
  (add `self.OnOpenCloseTorch` (delegate `OpenCloseTorch`))
  (set `self.NeedToBeHold` true))

(event `OpenCloseTorch`
  (`TimelineComponent.Stop` (`self.OpenClose`))
  (if (`self.IsOpen`)
    (set `self.IsOpen` false)
    (bind (_direction _alpha) (`Timeline|OpenClose` :!via `PlayFromStart` :!label _label)
      (:`Update`
        (`SceneComponent.K2_SetRelativeRotation` (`self.TorchTopContainter`) (`KismetMathLibrary.RLerp` (struct :`Roll` 140.0) (struct) _alpha) false false)))
    (else
      (set `self.IsOpen` true)
      (goto _label :!via `ReverseFromEnd`))))

(fn `Equip`
  (`parent.Equip`)
  (`SceneComponent.SetRelativeScale3D` (`self.ToolMesh`) (0.55 0.55 0.55))
  (if (not (`self.IsOpen`))
    (`self.OnOpenCloseTorch`)))

(fn `Unequip`
  (`parent.Unequip`)
  (`SceneComponent.SetRelativeScale3D` (`self.ToolMesh`) (0.4 0.4 0.4))
  (if (`self.IsOpen`)
    (`self.OnOpenCloseTorch`)))

(fn `Use`
  (bind _ns_fire (`self.NS_Fire`))
  (bind _heatsource (`self.HeatSource`))
  (`parent.Use`)
  (if (`self.IsOpen`)
    (`HeatSourceComponent.DeactivateSource` _heatsource)
    (`NiagaraComponent.ResetSystem` _ns_fire)
    (`NiagaraComponent.SetPaused` _ns_fire true)
    (else
      (`HeatSourceComponent.ActivateSource` _heatsource)
      (`NiagaraComponent.SetPaused` (`self.NS_Fire`) false)))
  (`self.OnOpenCloseTorch`))

(fn `UserConstructionScript`
  (`parent.UserConstructionScript`))