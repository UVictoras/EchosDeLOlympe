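; BP_DecorativeTorch is a torch actor with a Niagara fire effect and a point light that can be lit or put out.
; BeginPlay caches the light's intensity as BaseIntensity.
; SetFire activates the fire and restores that intensity, or deactivates it and zeroes the light.
; The IsOnAtStart check that would start the torch unlit is disconnected, so it never runs.
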(event `self.ReceiveBeginPlay`
  (set `self.BaseIntensity` (`LightComponentBase.Intensity` (`self.PointLight`))))

(fn `SetFire`
  (params (Value :type Boolean))
  (if Value
    (`ActorComponent.Activate` (`self.NS_Fire`) true)
    (`LightComponent.SetIntensity` (`self.PointLight`) (`self.BaseIntensity`))
    (else
      (`ActorComponent.Deactivate` (`self.NS_Fire`))
      (`LightComponent.SetIntensity` (`self.PointLight`) 0.0))))

(fn `UserConstructionScript`)