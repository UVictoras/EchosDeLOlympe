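; Manager for the Hephaistos forge puzzle, where lighting torches to match a random eight-bit code opens the Bassin.
; Activating the forge charges the first cable and loops hammer or sword sequences to show each bit, glowing between cycles.
; Torch updates are checked against the code, and any mismatch or forge deactivation resets the puzzle.
; Resets regenerate the code, keeping the first bit true, and lock blocked cables to later true-bit torches.
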(event `self.ReceiveBeginPlay`
  (`self.ResetEnigma`)
  (add `/Game/Blueprints/Interface/Interactibles/BP_Forge.OnActivateForge` (`self.Forge`) (delegate `StartEnigma`))
  (add `/Game/Blueprints/Interface/Interactibles/BP_Forge.OnDeactivateForge` (`self.Forge`) (delegate `StopEnigma`))
  (bind (_outactor _returnvalue) (`LevelSequencePlayer.CreateLevelSequencePlayer` (`self.HammerSequence`)))
  (set `self.HammerSequencePlayer` _returnvalue)
  (bind (_outactor_2 _returnvalue_2) (`LevelSequencePlayer.CreateLevelSequencePlayer` (`self.SwordSequence`)))
  (set `self.SwordSequencePlayer` _returnvalue_2)
  (for _array_element (`self.HephaistosTorches`)
    (add `/Game/Blueprints/Interface/Interactibles/BP_FlamableTorch.OnUpdateTorch` _array_element (`|CreateDelegate` :!event `UpdateCurrentCode`))))

(event `StartEnigma`
  (`/Game/Blueprints/Environment/BP_Cable.ChargeCable` (`self.FirstCable`))
  (`/Game/Blueprints/Interface/Interactibles/BP_FlamableTorch.SetFire` (`self.FirstTorch`) true)
  (`self.SequenceCycle`)
  (set `self.EnigmaPlaying` true))

(event `StopEnigma`
  (`self.ResetEnigma`)
  (`/Game/Blueprints/Interface/Interactibles/BP_Forge.SetFire` (`self.Forge`) false))

(event `SequenceCycle`
  (bind _hammersequenceplayer (`self.HammerSequencePlayer`))
  (bind _swordsequenceplayer (`self.SwordSequencePlayer`))
  (bind _returnvalue (`MovieSceneSequencePlayer.GetDuration` _hammersequenceplayer))
  (bind _returnvalue_2 (`MovieSceneSequencePlayer.GetDuration` _swordsequenceplayer))
  (if (`|GetArrayItem` (`self.Code`) (`self.CycleIndex`))
    (`MovieSceneSequencePlayer.Play` _hammersequenceplayer)
    (`KismetSystemLibrary.Delay` (+ (`KismetMathLibrary.Conv_IntToDouble` (/ (break `FrameNumber` (break `QualifiedFrameTime` _returnvalue)) (`KismetMathLibrary.BreakFrameRate` (`.FrameRate` (break `QualifiedFrameTime` _returnvalue))))) 0.25))
    (else
      (`MovieSceneSequencePlayer.Play` _swordsequenceplayer)
      (`KismetSystemLibrary.Delay` (+ (`KismetMathLibrary.Conv_IntToDouble` (/ (break `FrameNumber` (break `QualifiedFrameTime` _returnvalue_2)) (`KismetMathLibrary.BreakFrameRate` (`.FrameRate` (break `QualifiedFrameTime` _returnvalue_2))))) 0.25))))
  (bind _output_get (set `self.CycleIndex` (mod (+ 1 (`self.CycleIndex`)) 8)))
  (if (== 0 (mod _output_get 8))
    (`/Game/Blueprints/Interface/Interactibles/BP_Forge.Glow` (`self.Forge`))
    (`KismetSystemLibrary.Delay` 2.0)
    (`self.SequenceCycle` :!label _label)
    (elif (`self.EnigmaPlaying`)
      (goto _label))))

(fn `GenerateRandomCode`
  (bind _code (`self.Code`))
  (for (_ _array_index) _code
    (`KismetArrayLibrary.Array_Set` _code _array_index))
  (for (_ _array_index_2) (`self.Code`)
    (if (> _array_index_2 0)
      (if (and (== _array_index_2 7) (not (`KismetArrayLibrary.Array_Contains` (`self.Code`) true)))
        (`KismetArrayLibrary.Array_Set` (`self.Code`) 7 true)
        (else
          (`KismetArrayLibrary.Array_Set` (`self.Code`) _array_index_2 (`KismetMathLibrary.RandomBool`))))
      (`KismetArrayLibrary.Array_Set` (`self.CurrentCodeTry`) _array_index_2)))
  (`KismetArrayLibrary.Array_Set` (`self.Code`) 0 true))

(fn `ResetEnigma`
  (set `self.EnigmaPlaying` false)
  (`/Game/Blueprints/Interface/Interactibles/BP_Forge.SetFire` (`self.Forge`) false)
  (`self.GenerateRandomCode`)
  (for _array_element (`self.HephaistosTorches`)
    (`/Game/Blueprints/Interface/Interactibles/BP_FlamableTorch.SetFire` _array_element false)
    (`/Game/Blueprints/Environment/BP_Cable.DischargeCable` (`self.FirstCable`)))
  (for (_array_element_2 _array_index) (`self.BlockedCable`)
    (`/Game/Blueprints/Environment/BP_Cable.UnsetLocker` _array_element_2)
    (if true
      (for _index (range (+ _array_index 1) 8)
        (if (`|GetArrayItem` (`self.Code`) _index)
          (`/Game/Blueprints/Environment/BP_Cable.SetLocker` _array_element_2 (`|GetArrayItem` (`self.HephaistosTorches`) _index))
          (break))))))

(fn `UpdateCurrentCode`
  (params (Torch :type "/Game/Blueprints/Interface/Interactibles/BP_FlamableTorch Object Reference") (IsOnFire :type Boolean))
  (bind _returnvalue (`KismetArrayLibrary.Array_Find` (`self.HephaistosTorches`) Torch))
  (bind _output (`|GetArrayItem` (`self.Code`) _returnvalue))
  (if (== IsOnFire _output)
    (`KismetArrayLibrary.Array_Set` (`self.CurrentCodeTry`) _returnvalue _output)
    (`self.VerifyCode`)
    (else
      (`self.ResetEnigma`))))

(fn `UserConstructionScript`)

(fn `VerifyCode`
  (for (_array_element _array_index) (`self.CurrentCodeTry`)
    (if (not (== _array_element (`|GetArrayItem` (`self.Code`) _array_index)))
      (return)))
  (set `self.CodeFound` true)
  (for _array_element_2 (`self.HephaistosTorches`)
    (`/Game/Blueprints/Interface/Interactibles/BP_FlamableTorch.SetFire` _array_element_2 true)
    (`/Game/Blueprints/Interface/Interactibles/BP_FlamableTorch.DisableInteraction` _array_element_2))
  (`/Game/Blueprints/Interface/Interactibles/BP_Forge.DisableInteraction` (`self.Forge`))
  (`/Game/Blueprints/Environment/BP_Bassin.Open` (`self.Bassin`)))