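; Game instance that holds the player's tool loadout and last checkpoint for the rest of the game.
; Simple setters and getters store and return the tools and the current tool index.
; The checkpoint is kept as an actor reference, and its getter returns that actor's location, falling back to the player pawn's current location when the reference is invalid.
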(fn `GetCheckoint`
  (returns (checkpointLocation :type "Vector Structure"))
  (bind _checkpoint (`self.Checkpoint`))
  (`/Engine/EditorBlueprintResources/StandardMacros.IsValid` _checkpoint
    (:`Is Valid`
      (return (`Actor.K2_GetActorLocation` _checkpoint)))
    (:`Is Not Valid`
      (return (`Actor.K2_GetActorLocation` (`GameplayStatics.GetPlayerPawn` 0))))))

(fn `GetCurrentTool`
  (returns (Tool :type Integer))
  (return (`self.PlayerCurrentTooIndex`)))

(fn `GetTools`
  (returns (Tools :type "Array of /Game/Blueprints/Tools/BP_Tool Class Reference"))
  (return (`self.PlayerTools`)))

(fn `SetCurrentTools`
  (params (CurrentTool :type Integer))
  (set `self.PlayerCurrentTooIndex` CurrentTool))

(fn `SetLastCheckpoint`
  (params (Checkpoint :type "/Game/Blueprints/Trigger/BP_Checkpoint Object Reference"))
  (set `self.Checkpoint` Checkpoint))

(fn `SetPlayerTools`
  (params (Tool :type "Array of /Game/Blueprints/Tools/BP_Tool Class Reference"))
  (set `self.PlayerTools` Tool))