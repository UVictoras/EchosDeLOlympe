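; BP_Cable is a chainable cable section that carries a visible signal between linked neighbours.
; It relays charge and glow forward through events, while discharge requests travel onward so the chain drains back from the last charged section.
; Timelines drive material fill and emissive parameters, with fill rate divided by Z scale for consistent signal speed.
; An optional, swappable SignalBlocker holds incoming charge while locked and discharges a charged section upon locking.
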(event `self.ReceiveBeginPlay`
  (bind _previoussection (`self.PreviousSection`))
  (bind _signalblocker (`self.SignalBlocker`))
  (if (not (`self.IsFirstCable`))
    (add `self.OnGlow` (`self.PreviousSection`) (`|CreateDelegate` :!event `Glow`))
    (add `self.OnCharged` _previoussection (delegate `ChargeCable`))
    (add `self.OnNeedToDischarge` _previoussection (`|CreateDelegate` :!event `DischargeCable`))
    (`/Engine/EditorBlueprintResources/StandardMacros.IsValid` (`self.SignalBlocker`)
      (:`Is Valid`
        (add `/Game/Blueprints/Interface/Interactibles/BP_Lock.Lock` _signalblocker (`|CreateDelegate` :!event `BlockSignal`))
        (add `/Game/Blueprints/Interface/Interactibles/BP_Lock.Unlock` _signalblocker (`|CreateDelegate` :!event `UnblockSignal`))
        (set `self.IsSignalBlocked` true))
      (:`Is Not Valid`
        _)))
  (if (not (`self.IsLastCable`))
    (add `self.OnDischarged` (`self.NextSection`) (`|CreateDelegate` :!event `DischargeCable`))))

(event `ChargeCable`
  (bind (_returnvalue_x _returnvalue_y _returnvalue_z) (`KismetMathLibrary.BreakVector` (`self.GetActorScale3D`)))
  (`TimelineComponent.Stop` (`self.Discharge`))
  (if (`self.IsSignalBlocked`)
    (set `self.IsWaitingToCharge` true)
    (else
      (set `self.IsCableCharged` true)
      (`TimelineComponent.SetPlayRate` (`self.Charge`) (/ (`self.SignalSpeed`) _returnvalue_z))
      (bind (_direction _signalvalue) (`Timeline|Charge` :!via `PlayFromStart`)
        (:`Update`
          (`MeshComponent.SetScalarParameterValueOnMaterials` (`self.Cable`) "FillAmount" _signalvalue))
        (:`Finished`
          (`self.OnCharged`)
          (set `self.IsWaitingToCharge` false))))))

(event `DischargeCable`
  (bind (_relativescale3d_x _relativescale3d_y _relativescale3d_z) (`KismetMathLibrary.BreakVector` (`SceneComponent.RelativeScale3D` (`self.Cable`))))
  (`TimelineComponent.Stop` (`self.Charge`))
  (if (`self.IsCableCharged`)
    (if (`self.IsLastCable`)
      (set `self.IsCableCharged` false :!label _label)
      (`TimelineComponent.SetPlayRate` (`self.Discharge`) (/ (`self.SignalSpeed`) _relativescale3d_z))
      (bind (_direction _signalvalue) (`Timeline|Discharge` :!via `PlayFromStart`)
        (:`Update`
          (`MeshComponent.SetScalarParameterValueOnMaterials` (`self.Cable`) "FillAmount" _signalvalue))
        (:`Finished`
          (`self.OnDischarged`)
          (set `self.IsWaitingToDischarge` false)))
      (elif (`self.IsWaitingToDischarge`)
        (goto _label)
        (else
          (set `self.IsWaitingToDischarge` true)
          (`self.OnNeedToDischarge`))))
    (else
      (`self.OnDischarged`)
      (set `self.IsWaitingToCharge` false))))

(event `BlockSignal`
  (set `self.IsSignalBlocked` true)
  (if (`self.IsCableCharged`)
    (`self.DischargeCable`)))

(event `Glow`
  (bind _cable (`self.Cable`))
  (`self.OnGlow`)
  (bind (_direction _emissivevalue) (`Timeline|GlowSignal` :!via `PlayFromStart`)
    (:`Update`
      (`MeshComponent.SetScalarParameterValueOnMaterials` _cable "EmisiveScalar" _emissivevalue))
    (:`Finished`
      (bind (_direction_2 _emissivevalue_2) (`Timeline|NoGlowSignal` :!via `ReverseFromEnd`)
        (:`Update`
          (`MeshComponent.SetScalarParameterValueOnMaterials` _cable "EmisiveScalar" _emissivevalue_2))))))

(event `UnblockSignal`
  (set `self.IsSignalBlocked` false)
  (if (`self.IsWaitingToCharge`)
    (`self.ChargeCable`)
    (else
      (`KismetSystemLibrary.PrintString` "TARACELAPUT"))))

(fn `DebugChargeCable`
  (`self.ChargeCable`))

(fn `DebugNeedDischargeCable`
  (`self.DischargeCable`))

(fn `SetLocker`
  (params (`New Locker` :type "/Game/Blueprints/Interface/Interactibles/BP_Lock Object Reference"))
  (bind _output_get (set `self.SignalBlocker` `New Locker`))
  (`/Engine/EditorBlueprintResources/StandardMacros.IsValid` _output_get
    (:`Is Valid`
      (add `/Game/Blueprints/Interface/Interactibles/BP_Lock.Unlock` _output_get (`|CreateDelegate` :!event `UnblockSignal`))
      (add `/Game/Blueprints/Interface/Interactibles/BP_Lock.Lock` _output_get (`|CreateDelegate` :!event `BlockSignal`))
      (set `self.IsSignalBlocked` true))))

(fn `UnsetLocker`
  (bind _signalblocker (`self.SignalBlocker`))
  (set `self.IsSignalBlocked` false)
  (set `self.IsWaitingToCharge` false)
  (`/Engine/EditorBlueprintResources/StandardMacros.IsValid` _signalblocker
    (:`Is Valid`
      (remove `/Game/Blueprints/Interface/Interactibles/BP_Lock.Unlock` _signalblocker (`|CreateDelegate` :!event `UnblockSignal`))
      (remove `/Game/Blueprints/Interface/Interactibles/BP_Lock.Lock` _signalblocker (`|CreateDelegate` :!event `BlockSignal`))
      (set `self.SignalBlocker` null))))

(fn `UserConstructionScript`)