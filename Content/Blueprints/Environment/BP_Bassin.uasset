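; BP_Bassin is an environment basin that opens and lets the player exchange a torch for a Prometheus torch.
; Open sets IsOpen and plays a timeline that rotates the Scene component up to 120 degrees in yaw.
; Interact, only when open, swaps BP_Torch for BP_PrometheusTorch on the player, then disables further interaction by making Bottom ignore a custom trace channel.
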(event `Open`
  (set `self.IsOpen` true)
  (bind (_direction _alpha) (`Timeline|Timeline` :!via `PlayFromStart`)
    (:`Update`
      (`SceneComponent.K2_SetRelativeRotation` (`self.Scene`) (`KismetMathLibrary.RLerp` (struct) (struct :`Pitch` 120.0) _alpha) false false))))

(event `self.Interact`
  (params (Interactor :type "Actor Object Reference"))
  (if (`self.IsOpen`)
    (bind _asbp_player (cast `/Game/Blueprints/Player/BP_Player` Interactor))
    (`/Game/Blueprints/Player/BP_Player.LoseTool` _asbp_player "/Game/Blueprints/Tools/BP_Torch.BP_Torch_C")
    (`/Game/Blueprints/Player/BP_Player.GetTool` _asbp_player "/Game/Blueprints/Tools/BP_PrometheusTorch.BP_PrometheusTorch_C")
    (`self.DisableInteraction`)))

(fn `DisableInteraction`
  (`PrimitiveComponent.SetCollisionResponseToChannel` (`self.Bottom`) "ECC_GameTraceChannel1" "ECR_Ignore"))

(fn `UserConstructionScript`)