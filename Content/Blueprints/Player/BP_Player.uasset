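; Player character Blueprint that turns Enhanced Input actions into camera-relative movement, look, jump, hold-to-crouch, interaction and tool use.
; Interact sphere-traces ahead of the actor and sends InteractMessage to hit actors implementing the Interactible interface.
; GetTool spawns a tool, adds it to the Tools array and equips it.
; ChangeTool cycles or selects by index, moving tools between the hand socket and per-index belt sockets on the mesh.
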(event `self.ReceiveBeginPlay`)

(event `EnhancedInput|/Game/Inputs/Actions/IA_Move`
  (params (ActionValue :type "Vector2D Structure") (ElapsedSeconds :type "Float (double-precision)") (TriggeredSeconds :type "Float (double-precision)") (InputAction :type "InputAction Object Reference" :default "/Game/Inputs/Actions/IA_Move.IA_Move"))
  ;[0.6927 0 0 0.5] Inputs
  (:`Triggered`
    (`self.Move` ActionValue_X ActionValue_Y)))

(event `EnhancedInput|/Game/Inputs/Actions/IA_LookAround`
  (params (ActionValue :type "Vector2D Structure") (ElapsedSeconds :type "Float (double-precision)") (TriggeredSeconds :type "Float (double-precision)") (InputAction :type "InputAction Object Reference" :default "/Game/Inputs/Actions/IA_LookAround.IA_LookAround"))
  ;[0.6927 0 0 0.5] Inputs
  (:`Triggered`
    (`self.LookAround` ActionValue_X ActionValue_Y)))

(event `EnhancedInput|/Game/Inputs/Actions/IA_Jump`
  (params (ActionValue :type Boolean) (ElapsedSeconds :type "Float (double-precision)") (TriggeredSeconds :type "Float (double-precision)") (InputAction :type "InputAction Object Reference" :default "/Game/Inputs/Actions/IA_Jump.IA_Jump"))
  ;[0.6927 0 0 0.5] Inputs
  (:`Started`
    (`self.Jump`)))

(event `EnhancedInput|/Game/Inputs/Actions/IA_Crouch`
  (params (ActionValue :type Boolean) (ElapsedSeconds :type "Float (double-precision)") (TriggeredSeconds :type "Float (double-precision)") (InputAction :type "InputAction Object Reference" :default "/Game/Inputs/Actions/IA_Crouch.IA_Crouch"))
  ;[0.6927 0 0 0.5] Inputs
  (:`Started`
    (if (`NavMovementComponent.IsFalling` (`self.CharacterMovement`))
      (`self.UnCrouch` :!label _label)
      (else
        (`self.Crouch`))))
  (:`Completed`
    (goto _label)))

(event `EnhancedInput|/Game/Inputs/Actions/IA_Interact`
  (params (ActionValue :type Boolean) (ElapsedSeconds :type "Float (double-precision)") (TriggeredSeconds :type "Float (double-precision)") (InputAction :type "InputAction Object Reference" :default "/Game/Inputs/Actions/IA_Interact.IA_Interact"))
  ;[0.6927 0 0 0.5] Inputs
  (:`Started`
    (`self.Interact` ActionValue)))

(event `EnhancedInput|/Game/Inputs/Actions/IA_UseTool`
  (params (ActionValue :type Boolean) (ElapsedSeconds :type "Float (double-precision)") (TriggeredSeconds :type "Float (double-precision)") (InputAction :type "InputAction Object Reference" :default "/Game/Inputs/Actions/IA_UseTool.IA_UseTool"))
  ;[0.6927 0 0 0.5] Inputs
  (:`Triggered`
    (`/Engine/EditorBlueprintResources/StandardMacros.IsValid` (`self.CurrentTool`)
      (:`Is Valid`
        (`/Game/Blueprints/Tools/BP_Tool.Use` (`self.CurrentTool`))))))

(event `EnhancedInput|/Game/Inputs/Actions/IA_ChangeTool`
  (params (ActionValue :type Boolean) (ElapsedSeconds :type "Float (double-precision)") (TriggeredSeconds :type "Float (double-precision)") (InputAction :type "InputAction Object Reference" :default "/Game/Inputs/Actions/IA_ChangeTool.IA_ChangeTool"))
  ;[0.6927 0 0 0.5] Inputs
  (:`Started`
    (if (> (`KismetArrayLibrary.Array_Length` (`self.Tools`)) 1)
      (`self.ChangeTool` -1))))

(fn `ChangeTool`
  (params (Index :type Integer :default -1))
  (`self.Unequip`)
  (if (== -1 Index)
    (set `self.CurrentToolIndex` (mod (+ (`self.CurrentToolIndex`) 1) (`KismetArrayLibrary.Array_Length` (`self.Tools`))))
    (else
      (set `self.CurrentToolIndex` Index)))
  (`self.Equip`))

(fn `Equip`
  (bind _output_get (set `self.CurrentTool` (`|GetArrayItem` (`self.Tools`) (`self.CurrentToolIndex`))))
  (`/Game/Blueprints/Tools/BP_Tool.Equip` _output_get)
  (`self.K2_AttachToComponent` _output_get (`self.Mesh`) "HandSocket" "SnapToTarget" "SnapToTarget" "KeepRelative" true))

(fn `GetTool`
  (params (`Tool Class` :type "/Game/Blueprints/Tools/BP_Tool Class Reference"))
  (bind _returnvalue (`|SpawnActorFromClass` `Tool Class` (`KismetMathLibrary.MakeTransform` (0.0 0.0 0.0)) "AlwaysSpawn" "MultiplyWithRoot" self null))
  (bind _returnvalue_2 (`KismetArrayLibrary.Array_Add` (`self.Tools`) _returnvalue))
  (`self.ChangeTool` _returnvalue_2))

(fn `Interact`
  (params (InteractValue :type Boolean))
  (bind _returnvalue (`self.K2_GetActorLocation`))
  (bind _outhit (`KismetSystemLibrary.SphereTraceSingle` _returnvalue (+ _returnvalue (* (`self.GetActorForwardVector`) 150.0)) 100.0 "TraceTypeQuery3"))
  (bind (_bblockinghit _binitialoverlap _time _distance _location _impactpoint _normal _impactnormal _physmat _hitactor) (`GameplayStatics.BreakHitResult` _outhit))
  (if (`KismetSystemLibrary.DoesImplementInterface` _hitactor "/Script/EchosDeLOlympe.Interactible")
    (message `Interactible.Interact` _hitactor self)))

(fn `LookAround`
  (params (Yaw :type "Float (double-precision)") (Pitch :type "Float (double-precision)"))
  (bind _camerasensibility (`self.CameraSensibility`))
  (bind _result (`/Engine/EditorBlueprintResources/StandardMacros.NegateFloat` (* Yaw _camerasensibility))
    (:`  `
      (`self.AddControllerYawInput` _result)
      (`self.AddControllerPitchInput` (* Pitch _camerasensibility)))))

(fn `Move`
  (params (`Forward / Backward` :type "Float (double-precision)") (`Left / Right` :type "Float (double-precision)"))
  (bind (_returnvalue_roll _returnvalue_pitch _returnvalue_yaw) (`KismetMathLibrary.BreakRotator` (`self.GetControlRotation`)))
  (bind (_returnvalue_roll_2 _returnvalue_pitch_2 _returnvalue_yaw_2) (`KismetMathLibrary.BreakRotator` (`self.GetControlRotation`)))
  (`self.AddMovementInput` (`KismetMathLibrary.GetForwardVector` (`KismetMathLibrary.MakeRotator` 0.0 0.0 _returnvalue_yaw_2)) `Forward / Backward`)
  (`self.AddMovementInput` (`KismetMathLibrary.GetRightVector` (`KismetMathLibrary.MakeRotator` _returnvalue_roll 0.0 _returnvalue_yaw)) `Left / Right`))

(fn `Unequip`
  (bind _currenttool (`self.CurrentTool`))
  (`/Engine/EditorBlueprintResources/StandardMacros.IsValid` (`self.CurrentTool`)
    (:`Is Valid`
      (`/Game/Blueprints/Tools/BP_Tool.Unequip` _currenttool)
      (`self.K2_AttachToComponent` _currenttool (`self.Mesh`) (`|GetArrayItem` (`self.BeltsSocketNames`) (`self.CurrentToolIndex`)) "SnapToTarget" "SnapToTarget" "KeepRelative" true))))

(fn `UserConstructionScript`)