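; Double door that swings open once it is both unlocked and heat-activated.
; The Locker's unlock and the HeatReactor's react event share one opening path, so the conditions can be met in either order.
; A timeline rotates the two pivots 90 degrees in opposite directions.
; While closed, Tick fills two heat indicator materials with the HeatSubSystem temperature at the Sphere as a fraction of the reactor's activation temperature.
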(event `self.ReceiveBeginPlay`
  (add `/Game/Blueprints/Interactibles/BP_Lock.Unlock` (`self.Locker`) (delegate `CanOpen`))
  (`HeatReactor.Init` (`self.HeatReactor`)))

(event `CanOpen`
  (set `self.IsLocked` false)
  (if (`HeatReactor.IsReactorActive` (`self.HeatReactor`))
    (set `self.IsOpen` true :!label _label)
    (bind (_direction _alpha) (`Timeline|Timeline`)
      (:`Update`
        (`self.RotateDoor` (`KismetMathLibrary.NormalizeToRange` _alpha 0.0 1.0))))))

(event `self.HeatReactor.OnReact`
  (if (not (`self.IsLocked`))
    (goto _label)))

(event `self.ReceiveTick`
  (params (DeltaSeconds :type "Float (single-precision)"))
  (bind _returnvalue (/ (`HeatSubSystem.GetTemperatureAtLocation` (subsystem `HeatSubSystem`) (`SceneComponent.K2_GetComponentLocation` (`self.Sphere`))) (`HeatReactor.GetActivationTemperature` (`self.HeatReactor`))))
  (if (not (`self.IsOpen`))
    (`MeshComponent.SetScalarParameterValueOnMaterials` (`self.HeatIndicator`) "FillAmount" _returnvalue)
    (`MeshComponent.SetScalarParameterValueOnMaterials` (`self.HeatIndicator1`) "FillAmount" _returnvalue)))

(fn `RotateDoor`
  (params (RotatePercent :type "Float (double-precision)"))
  (`SceneComponent.K2_SetRelativeRotation` (`self.LeftPivot`) (`KismetMathLibrary.RLerp` (struct) (struct :`Yaw` -90.0) RotatePercent true) false false)
  (`SceneComponent.K2_SetRelativeRotation` (`self.RigthPivot`) (`KismetMathLibrary.RLerp` (struct) (struct :`Yaw` 90.0) RotatePercent true) false false))

(fn `UserConstructionScript`)