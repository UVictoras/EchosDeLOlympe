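; BP_MazePath is a maze path actor whose meshes glow while its HeatReactor is reacting.
; On BeginPlay it collects every static mesh component except the one named Plane into MazePath, then initializes HeatReactor.
; HeatReactor's react and stop-react events switch the EmissiveStrength material parameter on those meshes between a lit value and zero.
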(event `self.ReceiveBeginPlay`
  (for _array_element (`self.K2_GetComponentsByClass` "/Script/Engine.StaticMeshComponent")
    (if (not (`KismetStringLibrary.EqualEqual_StrStr` (`KismetSystemLibrary.GetObjectName` _array_element) "Plane"))
      (`KismetArrayLibrary.Array_Add` (`self.MazePath`) _array_element)))
  (`HeatReactor.Init` (`self.HeatReactor`)))

(event `self.HeatReactor.OnReact`
  (for _array_element (`self.MazePath`)
    (`MeshComponent.SetScalarParameterValueOnMaterials` _array_element "EmissiveStrength" 0.5)))

(event `self.HeatReactor.OnStopReact`
  (for _array_element (`self.MazePath`)
    (`MeshComponent.SetScalarParameterValueOnMaterials` _array_element "EmissiveStrength" 0.0)))

(fn `UserConstructionScript`)