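; BP_Enemy is an enemy whose AI activation depends on heat.
; At BeginPlay it compares the HeatSubSystem temperature at its location to the Reactor's activation temperature to seed the EnemyIsActive blackboard key.
; Reactor react and stop-react events then toggle that key.
; Tick drives HeatIndicator's FillAmount material parameter from the current-to-activation temperature ratio, while a timeline-based cooldown fill is left disconnected.
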(event `self.ReceiveBeginPlay`
  (bind __reactor (`self._reactor`))
  (`HeatReactor.Init` (`self._reactor`))
  (`BlackboardComponent.SetValueAsBool` (`AIBlueprintHelperLibrary.GetBlackboard` (`self.GetController`)) "EnemyIsActive" (>= (`HeatSubSystem.GetTemperatureAtLocation` (subsystem `HeatSubSystem`) (`self.K2_GetActorLocation`)) (`HeatReactor.GetActivationTemperature` (`self._reactor`))))
  (add `HeatReactor.OnReact` __reactor (delegate `SetActivateInBlackboard`))
  (add `HeatReactor.OnStopReact` __reactor (delegate `UnsetActivateInBlackboard`))
  (add `HeatReactor.OnCooling` (`self._reactor`) (`|CreateDelegate` :!event `SetIndicator`)))

(event `SetActivateInBlackboard`
  (`BlackboardComponent.SetValueAsBool` (`AIBlueprintHelperLibrary.GetBlackboard` (`self.GetController`)) "EnemyIsActive" true))

(event `UnsetActivateInBlackboard`
  (`BlackboardComponent.SetValueAsBool` (`AIBlueprintHelperLibrary.GetBlackboard` (`self.GetController`)) "EnemyIsActive" false))

(event `self.ReceiveTick`
  (params (DeltaSeconds :type "Float (single-precision)"))
  (bind __reactor (`self._reactor`))
  (`MeshComponent.SetScalarParameterValueOnMaterials` (`self.HeatIndicator`) "FillAmount" (/ (`HeatReactor.GetCurrentTemperature` __reactor) (`HeatReactor.GetActivationTemperature` __reactor))))

(event `SetIndicator`)

(fn `UserConstructionScript`)