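; Test enemy Blueprint that catches the player when its capsule hits a MainCharacter, calling GetCaught on that character.
; Escape and StopEscape switch the NeedToEscape blackboard key on and off, exposing flee state to the AI.
; An unconnected snippet that would set the IsStatic key never runs, and BeginPlay is empty.
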(event `self.ReceiveBeginPlay`)

(event `self.CapsuleComponent.OnComponentHit`
  (params (HitComponent :type "PrimitiveComponent Object Reference") (OtherActor :type "Actor Object Reference") (OtherComp :type "PrimitiveComponent Object Reference") (NormalImpulse :type "Vector Structure") (Hit :type "HitResult Structure (by ref)"))
  (bind _asmain_character (cast `MainCharacter` OtherActor))
  (`MainCharacter.GetCaught` _asmain_character))

(fn `Escape`
  (`BlackboardComponent.SetValueAsBool` (`AIBlueprintHelperLibrary.GetBlackboard` null) "NeedToEscape" true))

(fn `StopEscape`
  (`BlackboardComponent.SetValueAsBool` (`AIBlueprintHelperLibrary.GetBlackboard` null) "NeedToEscape" false))

(fn `UserConstructionScript`)