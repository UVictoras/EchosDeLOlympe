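; BP_FlamableTorch is an interactable torch that toggles fire on and off and drives a lock.
; SetFire switches the Niagara fire and restores or zeroes the point light's cached intensity.
; Each interaction broadcasts the torch state, then calls lock or unlock according to IsUnlockWhenOn.
; A HeatSource is initialized at start and deactivated if the torch starts unlit; collision-channel responses enable or disable interaction.
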(event `self.ReceiveBeginPlay`
  (`HeatSourceComponent.Init` (`self.HeatSource`))
  (set `self.BaseIntensity` (`LightComponentBase.Intensity` (`self.PointLight`)))
  (if (not (`self.IsUnlockWhenOn`))
    (`self.Unlock`))
  (if (not (`self.IsOnAtStart`))
    (`ActorComponent.Deactivate` (`self.NS_Fire`))
    (`LightComponent.SetIntensity` (`self.PointLight`) 0.0)
    (`HeatSourceComponent.DeactivateSource` (`self.HeatSource`))))

(event `self.Interact`
  (params (Interactor :type "Actor Object Reference"))
  (bind _isunlockwhenon (`self.IsUnlockWhenOn`))
  (`self.SetFire` (not (`self.IsOnFire`)))
  (`self.OnUpdateTorch` self (`self.IsOnFire`))
  (if (`self.IsOnFire`)
    (if _isunlockwhenon
      (`self.Unlock`)
      (else
        (`self.Lock` :!label _label)))
    (elif _isunlockwhenon
      (goto _label)
      (else
        (`self.Unlock`)))))

(fn `DisableInteraction`
  (`PrimitiveComponent.SetCollisionResponseToChannel` (`self.Torch`) "ECC_GameTraceChannel1" "ECR_Ignore"))

(fn `EnableInteraction`
  (`PrimitiveComponent.SetCollisionResponseToChannel` (`self.Torch`) "ECC_GameTraceChannel1" "ECR_Block"))

(fn `GetStatus`
  (returns (IsOnFire :type Boolean))
  (return (`self.IsOnFire`)))

(fn `SetFire`
  (params (Value :type Boolean))
  (if Value
    (`ActorComponent.Activate` (`self.NS_Fire`) true)
    (`LightComponent.SetIntensity` (`self.PointLight`) (`self.BaseIntensity`))
    (set `self.IsOnFire` true)
    (else
      (`ActorComponent.Deactivate` (`self.NS_Fire`))
      (`LightComponent.SetIntensity` (`self.PointLight`) 0.0)
      (set `self.IsOnFire` false))))

(fn `UserConstructionScript`)