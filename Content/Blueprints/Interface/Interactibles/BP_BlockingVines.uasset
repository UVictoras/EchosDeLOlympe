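; BP_BlockingVines is an interactable vine obstacle that the player burns away with a torch.
; On Interact it checks that the BP_Player holds BP_Torch, then starts the dissolve and blocks repeat interactions.
; A timeline drives the DissolveAmount material parameter on the plane mesh, then fires CallUnlock and destroys the actor when it finishes.
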(event `self.ReceiveBeginPlay`)

(event `self.Interact`
  (params (Interactor :type "Actor Object Reference"))
  (if (not (`self.IsDisolving`))
    (bind _asbp_player (cast `/Game/Blueprints/Player/BP_Player` Interactor))
    (bind _hastool (`/Game/Blueprints/Player/BP_Player.PlayerHasTool` _asbp_player "/Game/Blueprints/Tools/BP_Torch.BP_Torch_C"))
    (if _hastool
      (`self.DissolveVine`)
      (set `self.IsDisolving` true))))

(event `DissolveVine`
  (bind (_direction _dissolvetrack) (`Timeline|Dissolve` :!via `PlayFromStart`)
    (:`Update`
      (`MeshComponent.SetScalarParameterValueOnMaterials` (`self.Plane`) "DissolveAmount" _dissolvetrack))
    (:`Finished`
      (`self.Unlock`)
      (`self.K2_DestroyActor`))))

(fn `UserConstructionScript`)