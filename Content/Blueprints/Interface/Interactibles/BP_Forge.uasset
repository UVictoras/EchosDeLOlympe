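; Interactible forge that toggles its fire effect and point light, calling unlock or lock along with activate or deactivate events.
; The Hammer's anvil-hit event is bound to make the first cable glow, starting a signal.
; The forge's own Glow event chains two timelines to pulse the light intensity.
; Interaction is enabled or disabled by switching the forge mesh's response on a custom trace channel.
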(event `self.ReceiveBeginPlay`
  (bind _pointlight (`self.PointLight`))
  (`parent.ReceiveBeginPlay`)
  (`ActorComponent.Deactivate` (`self.NS_Fire`))
  (set `self.BaseIntensity` (`LightComponentBase.Intensity` _pointlight))
  (`LightComponent.SetIntensity` _pointlight 0.0)
  (add `/Game/Blueprints/Environment/BP_Hammer.OnHitAnvil` (`self.Hammer`) (delegate `MakeSignalGlow`)))

(event `MakeSignalGlow`
  (`/Game/Blueprints/Environment/BP_Cable.Glow` (`self.FirstCable`)))

(event `self.Interact`
  (params (Interactor :type "Actor Object Reference"))
  (`self.SetFire` (not (`self.IsOnFire`)))
  (if (`self.IsOnFire`)
    (`self.Unlock`)
    (`self.OnActivateForge`)
    (else
      (`self.Lock`)
      (`self.OnDeactivateForge`))))

(event `Glow`
  (bind (_direction _intensity) (`Timeline|FireGlow` :!via `PlayFromStart`)
    (:`Update`
      (`LightComponent.SetIntensity` (`self.PointLight`) _intensity))
    (:`Finished`
      (bind (_direction_2 _intensity_2) (`Timeline|RemoveGlow` :!via `PlayFromStart`)
        (:`Update`
          (`LightComponent.SetIntensity` (`self.PointLight`) _intensity_2))))))

(fn `DisableInteraction`
  (`PrimitiveComponent.SetCollisionResponseToChannel` (`self.Forge`) "ECC_GameTraceChannel1" "ECR_Ignore"))

(fn `EnableInteraction`
  (`PrimitiveComponent.SetCollisionResponseToChannel` (`self.Forge`) "ECC_GameTraceChannel1" "ECR_Block"))

(fn `SetFire`
  (params (IsOnFire :type Boolean))
  (if IsOnFire
    (`ActorComponent.Activate` (`self.NS_Fire`) true)
    (`LightComponent.SetIntensity` (`self.PointLight`) (`self.BaseIntensity`))
    (set `self.IsOnFire` true)
    (else
      (`ActorComponent.Deactivate` (`self.NS_Fire`))
      (`LightComponent.SetIntensity` (`self.PointLight`) 0.0)
      (set `self.IsOnFire` false))))

(fn `UserConstructionScript`
  (`parent.UserConstructionScript`))