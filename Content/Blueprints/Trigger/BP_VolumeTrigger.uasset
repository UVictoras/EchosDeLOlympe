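; BP_VolumeTrigger is a trigger that fades the volume of a referenced Sound's audio component as the player enters and leaves.
; On overlap with BP_Player, the VolumeDown timeline plays from the start and drives the component's volume multiplier.
; When the player leaves, a separate timeline plays in reverse from its end to drive the same multiplier.
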(event `self.ReceiveActorBeginOverlap`
  (params (OtherActor :type "Actor Object Reference"))
  (cast `/Game/Blueprints/Player/BP_Player` OtherActor)
  (bind (_direction _newtrack_0) (`Timeline|VolumeDown` :!via `PlayFromStart`)
    (:`Update`
      (`AudioComponent.SetVolumeMultiplier` (`AmbientSound.AudioComponent` (`self.Sound`)) _newtrack_0))))

(event `self.Box.OnComponentBeginOverlap`
  (params (OverlappedComponent :type "PrimitiveComponent Object Reference") (OtherActor :type "Actor Object Reference") (OtherComp :type "PrimitiveComponent Object Reference") (OtherBodyIndex :type Integer) (bFromSweep :type Boolean) (SweepResult :type "HitResult Structure (by ref)")))

(event `self.ReceiveActorEndOverlap`
  (params (OtherActor :type "Actor Object Reference"))
  (cast `/Game/Blueprints/Player/BP_Player` OtherActor)
  (bind (_direction _newtrack_0) (`Timeline|Timeline` :!via `ReverseFromEnd`)
    (:`Update`
      (`AudioComponent.SetVolumeMultiplier` (`AmbientSound.AudioComponent` (`self.Sound`)) _newtrack_0))))

(fn `UserConstructionScript`)