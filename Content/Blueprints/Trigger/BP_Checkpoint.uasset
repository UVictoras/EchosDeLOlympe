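; BP_Checkpoint is a trigger that records itself as the last checkpoint when the player reaches it.
; Overlapping its Box with a BP_Player passes the checkpoint actor to SetLastCheckpoint on BP_EdlOGameInstance.
; A checkpoint flagged IsDefault also registers itself on BeginPlay, providing the initial checkpoint.
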(event `self.ReceiveBeginPlay`
  (if (`self.isDefault`)
    (bind _asbp_edl_ogame_instance (cast `/Game/Blueprints/Game/BP_EdlOGameInstance` (`GameplayStatics.GetGameInstance`)))
    (`/Game/Blueprints/Game/BP_EdlOGameInstance.SetLastCheckpoint` _asbp_edl_ogame_instance self)))

(event `self.Box.OnComponentBeginOverlap`
  (params (OverlappedComponent :type "PrimitiveComponent Object Reference") (OtherActor :type "Actor Object Reference") (OtherComp :type "PrimitiveComponent Object Reference") (OtherBodyIndex :type Integer) (bFromSweep :type Boolean) (SweepResult :type "HitResult Structure (by ref)"))
  (cast `/Game/Blueprints/Player/BP_Player` OtherActor)
  (bind _asbp_edl_ogame_instance (cast `/Game/Blueprints/Game/BP_EdlOGameInstance` (`GameplayStatics.GetGameInstance`)))
  (`/Game/Blueprints/Game/BP_EdlOGameInstance.SetLastCheckpoint` _asbp_edl_ogame_instance self))

(fn `UserConstructionScript`
  (`parent.UserConstructionScript`))