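; BP_UITrigger is a one-shot trigger actor that shows a UI widget while the player overlaps it.
; On begin overlap with BP_Player, it creates the configurable WidgetToSpawn class, stores the instance and adds it to the viewport.
; On end overlap, RemoveUI takes the widget off screen and destroys the trigger, provided the widget is valid.
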(event `self.ReceiveActorBeginOverlap`
  (params (OtherActor :type "Actor Object Reference"))
  (bind _widgettospawn (`self.WidgetToSpawn`))
  (cast `/Game/Blueprints/Player/BP_Player` OtherActor)
  (if (`KismetSystemLibrary.IsValidClass` _widgettospawn)
    (bind _returnvalue (`|CreateWidget` _widgettospawn))
    (bind _output_get (set `self.WidgetCreated` _returnvalue))
    (`UserWidget.AddToViewport` _output_get 0)))

(event `self.ReceiveActorEndOverlap`
  (params (OtherActor :type "Actor Object Reference"))
  (cast `/Game/Blueprints/Player/BP_Player` OtherActor)
  (`self.RemoveUI`))

(event `RemoveUI`
  (bind _widgetcreated (`self.WidgetCreated`)
    (:`then`
      (`Widget.RemoveFromParent` _widgetcreated)
      (`self.K2_DestroyActor`))
    (:`else`)))

(fn `UserConstructionScript`)